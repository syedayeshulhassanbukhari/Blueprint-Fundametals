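; Night lighting controller Blueprint that switches the level's lighting to a moonlit night look at BeginPlay.
; It finds the DirectionalLight, SkyLight and PostProcessVolume by class, dims and blue-tints both lights, angles the directional light and recaptures the sky.
; The post-process volume stays unchanged; a debug message flags exposure bias for manual adjustment, and another reports completion.
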(event `self.ReceiveBeginPlay`
  (`|ExecutionSequence`
    (:`then_0`
      (bind _returnvalue (`GameplayStatics.GetActorOfClass` "/Script/Engine.DirectionalLight"))
      (bind _output_get (set `self.DirectionalLight` _returnvalue))
      (bind _returnvalue_2 (`GameplayStatics.GetActorOfClass` "/Script/Engine.SkyLight"))
      (bind _output_get_2 (set `self.SkyLight` _returnvalue_2))
      (bind _returnvalue_3 (`GameplayStatics.GetActorOfClass` "/Script/Engine.PostProcessVolume"))
      (bind _output_get_3 (set `self.PostProcessVolume` _returnvalue_3))
      (bind _returnvalue_4 (`self.GetComponentByClass` _output_get "/Script/Engine.LightComponent"))
      (`LightComponent.SetIntensity` _returnvalue_4 0.15)
      (`LightComponent.SetLightColor` _returnvalue_4 (`KismetMathLibrary.MakeColor` 0.6 0.7 1.0) true)
      (`self.K2_SetActorRotation` _output_get (`KismetMathLibrary.MakeRotator` 0.0 -45.0 180.0) false)
      (bind _returnvalue_5 (`self.GetComponentByClass` _output_get_2 "/Script/Engine.SkyLightComponent"))
      (`SkyLightComponent.SetIntensity` _returnvalue_5 0.05)
      (`SkyLightComponent.SetLightColor` _returnvalue_5 (`KismetMathLibrary.MakeColor` 0.4 0.5 0.8))
      (`SkyLightComponent.RecaptureSky` _returnvalue_5)
      (`/Engine/EditorBlueprintResources/StandardMacros.IsValid` _output_get_3
        (:`Is Valid`
          (`KismetSystemLibrary.PrintString` "PostProcessVolume found - manual adjustment needed for AutoExposureBias" true true (struct :`G` 0.66 :`B` 1.0 :`A` 1.0) 5.0))))
    (:`then_1`
      (`KismetSystemLibrary.PrintString` "Night Lighting Applied Successfully" true true (`KismetMathLibrary.MakeColor` 0.0 0.0 1.0) 5.0))))

(event `self.ReceiveActorBeginOverlap`
  (params (OtherActor :type "Actor Object Reference")))

(event `self.ReceiveTick`
  (params (DeltaSeconds :type "Float (single-precision)")))

(fn `UserConstructionScript`)