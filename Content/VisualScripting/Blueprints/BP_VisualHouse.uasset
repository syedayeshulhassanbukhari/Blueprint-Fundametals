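; BP_VisualHouse is a Blueprint scripting exercise covering functions, custom events, maps, arrays and runtime component creation.
; BeginPlay runs only the function demos: a printed intro and an addition whose result is unused.
; StartEvents, which nothing here calls, chains the event, map and array demos into a house build.
; That build adds static mesh components at fixed transforms: cubes for floor and walls, ramps for the roof.
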(event `self.ReceiveBeginPlay`
  (`self.Event StartFunctions`))

(event `Event StartFunctions`
  ; Functions added into the event graph
  (`self.Intro to Function`)
  (`self.addTwoNumbers` 2.6 1.4))

(event `Event StartEvents`
  ; Custom Event List
  (`self.Event DoStuff`)
  (`self.Event Map Weapons`)
  (`self.Event Add Fruits to Baskets`)
  (`self.Event Build House in real Time`))

(event `Event Map Weapons`
  ; Understanding Maps
  (`KismetSystemLibrary.PrintString` (`KismetStringLibrary.Conv_IntToString` (`BlueprintMapLibrary.Map_Find` (`self.Weapons`) (`self.Mapping in Weapons`))))
  (`BlueprintMapLibrary.Map_Add` (`self.Weapons`) "Knife" 1)
  (`KismetSystemLibrary.PrintString` (`KismetStringLibrary.Conv_IntToString` (`BlueprintMapLibrary.Map_Find` (`self.Weapons`) "Knife"))))

(event `Event DoStuff`
  ; Undertanding Custom Events
  (`KismetSystemLibrary.PrintString` "Custom Event Activated"))

(event `Event Add Fruits to Baskets`
  ; Understanding Array
  (`KismetSystemLibrary.PrintString` (`|GetArrayItem` (`self.Fruits Bucket`)))
  (`KismetArrayLibrary.Array_Set` (`self.Fruits Bucket`) 4 "Kiwi")
  (`KismetSystemLibrary.PrintString` (`|GetArrayItem` (`self.Fruits Bucket`) (`self.Fruit Bucket Index`)))
  (set `self.Fruits Bucket` (`|MakeArray` "Blueberries"))
  (`KismetSystemLibrary.PrintString` (`|GetArrayItem` (`self.Fruits Bucket`))))

(event `Event Build House in real Time`
  ; Set foundation for house
  (`KismetSystemLibrary.PrintString` "Start Construction")
  (bind _returnvalue (`AddComponent|NODE_AddStaticMeshComponent-0`))
  (`StaticMeshComponent.SetStaticMesh` _returnvalue "/Engine/BasicShapes/Cube.Cube")
  (`SceneComponent.K2_SetRelativeLocation` _returnvalue (0.0 0.0 0.0) false false)
  (`SceneComponent.SetRelativeScale3D` _returnvalue (1.0 1.0 0.05))
  ; Constructing Walls
  (bind _returnvalue_2 (`AddComponent|NODE_AddStaticMeshComponent-1` :`RelativeTransform` (`KismetMathLibrary.MakeTransform` (35.0 0.0 27.700396) (struct) (0.05 0.5 0.5))))
  (`StaticMeshComponent.SetStaticMesh` _returnvalue_2 "/Engine/BasicShapes/Cube.Cube")
  (bind _returnvalue_3 (`AddComponent|NODE_AddStaticMeshComponent-2` :`RelativeTransform` (`KismetMathLibrary.MakeTransform` (-35.0 0.0 27.700396) (struct) (0.05 0.5 0.5))))
  (`StaticMeshComponent.SetStaticMesh` _returnvalue_3 "/Engine/BasicShapes/Cube.Cube")
  (bind _returnvalue_4 (`AddComponent|NODE_AddStaticMeshComponent-3` :`RelativeTransform` (`KismetMathLibrary.MakeTransform` (-0.074336 27.061056 27.700396) (struct :`Yaw` 89.999999) (0.05 0.75 0.5))))
  (`StaticMeshComponent.SetStaticMesh` _returnvalue_4 "/Engine/BasicShapes/Cube.Cube")
  (bind _returnvalue_5 (`AddComponent|NODE_AddStaticMeshComponent-4` :`RelativeTransform` (`KismetMathLibrary.MakeTransform` (-0.074336 -26.950243 27.700396) (struct :`Yaw` -89.0) (0.05 0.75 0.5))))
  (`StaticMeshComponent.SetStaticMesh` _returnvalue_5 "/Engine/BasicShapes/Cube.Cube")
  ; Constructing Roof Tops
  (bind _returnvalue_6 (`AddComponent|NODE_AddStaticMeshComponent-5` :`RelativeTransform` (`KismetMathLibrary.MakeTransform` (39.852356 -0.379747 53.232509) (struct :`Yaw` -179.0) (0.8 0.4 0.4))))
  (`StaticMeshComponent.SetStaticMesh` _returnvalue_6 "/Game/LevelPrototyping/Meshes/SM_Ramp.SM_Ramp")
  (bind _returnvalue_7 (`AddComponent|NODE_AddStaticMeshComponent-6` :`RelativeTransform` (`KismetMathLibrary.MakeTransform` (-39.849471 0.0 53.23251) (struct) (0.8 0.4 0.4))))
  (`StaticMeshComponent.SetStaticMesh` _returnvalue_7 "/Game/LevelPrototyping/Meshes/SM_Ramp.SM_Ramp"))

(fn `addTwoNumbers`
  (params (varFirst :type "Float (double-precision)") (VarSecond :type "Float (double-precision)"))
  (returns (ResultVar :type "Float (double-precision)"))
  ; Passing Parameters into the function
  (return (+ varFirst VarSecond)))

(fn `Intro to Function`
  (`KismetSystemLibrary.PrintString` "Custom Functions Created is being started" true true (struct :`R` 1.0 :`G` 0.077124 :`B` 0.041784 :`A` 1.0)))

(fn `UserConstructionScript`)