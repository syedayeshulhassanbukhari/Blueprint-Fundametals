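; BP_VisualHouse is a visual scripting practice Blueprint that experiments with maps, arrays and procedural component creation.
; BeginPlay prints a lookup from the Weapons map, adds a Knife entry and prints its value.
; An unconnected chain would build a small house from scaled cube and ramp static mesh components added at runtime.
; A second unconnected chain demonstrates array reads and writes on FruitsBucket, and the construction script is empty.
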(event `self.ReceiveBeginPlay`
  (`KismetSystemLibrary.PrintString` (`KismetStringLibrary.Conv_IntToString` (`BlueprintMapLibrary.Map_Find` (`self.Weapons`) (`self.Mapping in Weapons`))))
  (`BlueprintMapLibrary.Map_Add` (`self.Weapons`) "Knife" 1)
  (`KismetSystemLibrary.PrintString` (`KismetStringLibrary.Conv_IntToString` (`BlueprintMapLibrary.Map_Find` (`self.Weapons`) "Knife"))))

(fn `UserConstructionScript`)