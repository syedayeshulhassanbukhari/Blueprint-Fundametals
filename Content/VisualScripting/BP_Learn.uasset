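; BP_Learn is a practice Blueprint for rehearsing common nodes and access to components from the Viewport.
; On BeginPlay it prints messages, draws a debug sphere and spawns a tutorial particle emitter at fixed locations.
; A chain of Delay nodes then steps world-offset moves on the spawned emitter, the Plane component and the BallStaticMesh component in sequence.
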(event `self.ReceiveBeginPlay`
  ; Buiding Muscle Memory for different Nodes in Blueprints with accessing Components from Viewport
  (`KismetSystemLibrary.PrintString` "Hello")
  (`KismetSystemLibrary.PrintString` "World !" true true (struct :`R` 0.99964 :`G` 0.237346 :`B` 1.0 :`A` 1.0))
  (`KismetSystemLibrary.DrawDebugSphere` (-50.0 -1250.0 50.0) 100.0 12 (struct :`R` 1.0 :`G` 1.0 :`B` 1.0 :`A` 1.0) (`self.Duration`))
  (bind _returnvalue (`GameplayStatics.SpawnEmitterAtLocation` "/Engine/Tutorial/SubEditors/TutorialAssets/TutorialParticleSystem.TutorialParticleSystem" (-100.0 -1300.0 50.0)))
  (`KismetSystemLibrary.Delay` 2.0)
  (`SceneComponent.K2_AddWorldOffset` _returnvalue (0.0 200.0 0.0) false false)
  (`KismetSystemLibrary.Delay` 2.0)
  (`SceneComponent.K2_AddWorldOffset` _returnvalue (0.0 150.0 0.0) false false)
  (`KismetSystemLibrary.Delay` 0.2)
  (`SceneComponent.K2_AddWorldOffset` (`self.Plane`) (0.0 0.0 250.0) false false)
  (`KismetSystemLibrary.Delay` 0.2)
  (`SceneComponent.K2_AddWorldOffset` (`self.BallStaticMesh`) (250.0 0.0 0.0) false false))

(fn `UserConstructionScript`)